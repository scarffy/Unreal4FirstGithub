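; Game instance that sets the PlayFab title ID on init and handles player account requests.
; Signup, Login and ForgotPassword events send PlayFab client calls for registration, email login and account recovery.
; Successful signup or login opens the PostPlayfabLogin level, while a sent recovery email prints a confirmation.
; Registration failures print the error name, message and details on screen in red.
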(event `self.ReceiveInit`
  (`PlayFabUtilities.setPlayFabSettings` (`self.GameId`)))

(event `OnRegisterSuccess`
  (params (result :type "ClientRegisterPlayFabUserResult Structure") (customData :type "Object Object Reference"))
  (`GameplayStatics.OpenLevelBySoftObjectPtr` "/Game/Maps/PostPlayfabLogin.PostPlayfabLogin"))

(event `Signup`
  (params (Username :type String) (Email :type String) (Password :type String))
  ;[1 1 1] Register
  (`PlayFabClientAPI.RegisterPlayFabUser` (make `ClientRegisterPlayFabUserRequest` null Username Email "" null Password "" true Username) (delegate `OnRegisterSuccess`) (delegate `OnFail`)))

(event `OnFail`
  (params (error :type "PlayFabError Structure") (customData :type "Object Object Reference"))
  ;[1 1 1] Register
  (`KismetSystemLibrary.PrintString` (`KismetStringLibrary.Concat_StrStr` error_ErrorName ":" error_ErrorMessage "(" error_ErrorDetails ").") true true (struct :`R` 1.0 :`B` 0.152896 :`A` 1.0) 10.0))

(event `Login`
  (params (Email :type String) (Password :type String))
  ;[1 1 1] Login
  (`PlayFabClientAPI.LoginWithEmailAddress` (make `ClientLoginWithEmailAddressRequest` null Email null Password) (delegate `OnLoginSuccess`) (`|CreateDelegate` :!event `OnFail`)))

(event `OnLoginSuccess`
  (params (result :type "ClientLoginResult Structure") (customData :type "Object Object Reference"))
  ;[1 1 1] Login
  (`GameplayStatics.OpenLevelBySoftObjectPtr` "/Game/Maps/PostPlayfabLogin.PostPlayfabLogin"))

(event `ForgotPassword`
  (params (Email :type String))
  ;[1 1 1] Forgot Password
  (`PlayFabClientAPI.SendAccountRecoveryEmail` (make `ClientSendAccountRecoveryEmailRequest` null Email) (delegate `RecoveryEmailSuccess`) (`|CreateDelegate` :!event `OnFail`)))

(event `RecoveryEmailSuccess`
  (params (result :type "ClientSendAccountRecoveryEmailResult Structure") (customData :type "Object Object Reference"))
  ;[1 1 1] Forgot Password
  (`KismetSystemLibrary.PrintString` "A recovery email has been sent" true true (struct :`G` 0.66 :`B` 1.0 :`A` 1.0) 10.0))